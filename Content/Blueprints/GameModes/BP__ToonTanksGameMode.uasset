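; Game mode Blueprint for Toon Tanks that handles the start and end-of-match screens.
; StartGame shows the start widget, then removes all widgets after a fixed delay.
; GameOver shows the win/lose widget and sets its text from the WonGame flag.
; BeginPlay, Tick and the construction script are empty.
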(event EventBeginPlay)

(event EventTick
  (params (DeltaSeconds :type Float%20%28single-precision%29)))

(event EventStartGame
  (bind _returnvalue (UserInterface|CreateWidget "/Game/Blueprints/Widgets/wbp_startWidget.wbp_startWidget_C"))
  (UserInterface|Viewport|AddtoViewport _returnvalue 0)
  (Utilities|FlowControl|Delay 4.0)
  (Viewport|RemoveAllWidgets))

(event EventGameOver
  (params (bWonGame :type Boolean))
  (bind _returnvalue (UserInterface|CreateWidget "/Game/Blueprints/Widgets/wbp_WinLose.wbp_WinLose_C"))
  (UserInterface|Viewport|AddtoViewport _returnvalue 0)
  (if bWonGame
    (Rendering|Components|TextRender|SetText (Variables|/Game/Blueprints/Widgets/wbp_WinLose.wbp_WinLose_C|GetDisplayText _returnvalue) "You  Won !!!")
    (else
      (Rendering|Components|TextRender|SetText (Variables|/Game/Blueprints/Widgets/wbp_WinLose.wbp_WinLose_C|GetDisplayText _returnvalue) "You Lost !!!"))))

(fn ConstructionScript)